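; Enemy AI character that fights with sword combos, can be stealth-killed from behind, and shows camera-facing health, kill and investigate widgets.
; Attack calls, apparently from a behavior tree, chain montages through a saved-attack index, while timer-looped sphere traces damage "Damagable" actors.
; Damage interrupts combos, launches the enemy and feeds BPCPlayerStats; death triggers ragdoll and notifies the player's quest component.
; StealthBackKill plays a paired victim montage, ragdolls, and returns alignment data.
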(event `self.ReceiveBeginPlay`
  ;[1 1 1] Getting the health bar
  (bind _aswb_dummy_health_bar (cast `/Game/UI/WB_DummyHealthBar` (`WidgetComponent.GetWidget` (`self.Health Bar Widget`))))
  (set `self.Health Bar UI` _aswb_dummy_health_bar))

(event `self.ReceiveTick`
  (params (DeltaSeconds :type "Float (single-precision)"))
  ;[0 0.2755 1] Setting rotation
  (`SceneComponent.K2_SetWorldRotation` (`self.Kill Widget`) (`KismetMathLibrary.FindLookAtRotation` (`SceneComponent.K2_GetComponentLocation` (`self.Kill Widget`)) (`SceneComponent.K2_GetComponentLocation` (`PlayerCameraManager.TransformComponent` (`GameplayStatics.GetPlayerCameraManager` 0)))) false false)
  (`SceneComponent.K2_SetWorldRotation` (`self.Health Bar Widget`) (`KismetMathLibrary.FindLookAtRotation` (`SceneComponent.K2_GetComponentLocation` (`self.Kill Widget`)) (`SceneComponent.K2_GetComponentLocation` (`PlayerCameraManager.TransformComponent` (`GameplayStatics.GetPlayerCameraManager` 0)))) false false)
  (`SceneComponent.K2_SetWorldRotation` (`self.Investigate Widget`) (`KismetMathLibrary.FindLookAtRotation` (`SceneComponent.K2_GetComponentLocation` (`self.Kill Widget`)) (`SceneComponent.K2_GetComponentLocation` (`PlayerCameraManager.TransformComponent` (`GameplayStatics.GetPlayerCameraManager` 0)))) false false))

(event `self.KillRadius.OnComponentBeginOverlap`
  (params (OverlappedComponent :type "PrimitiveComponent Object Reference") (OtherActor :type "Actor Object Reference") (OtherComp :type "PrimitiveComponent Object Reference") (OtherBodyIndex :type Integer) (bFromSweep :type Boolean) (SweepResult :type "HitResult Structure (by ref)"))
  ;[0.2601 0.5652 1] Setting visibility when dead
  (cast `/Game/ThirdPerson/Blueprints/BP_ThirdPersonCharacter` OtherActor)
  (`SceneComponent.SetVisibility` (`self.Kill Widget`) true false))

(event `self.KillRadius.OnComponentEndOverlap`
  (params (OverlappedComponent :type "PrimitiveComponent Object Reference") (OtherActor :type "Actor Object Reference") (OtherComp :type "PrimitiveComponent Object Reference") (OtherBodyIndex :type Integer))
  ;[0.2601 0.5652 1] Setting visibility when dead
  (cast `/Game/ThirdPerson/Blueprints/BP_ThirdPersonCharacter` OtherActor)
  (`SceneComponent.SetVisibility` (`self.Kill Widget`) false false))

(event `RagDoll`
  ;[0 1 0.8298] Ragdoll
  (`|ExecutionSequence`
    (:`then_0`
      (`KismetSystemLibrary.Delay` 2.5)
      (`PrimitiveComponent.SetSimulatePhysics` (`self.Mesh`) true)
      (`KismetSystemLibrary.Delay` 2.5))
    (:`then_1`
      (`KismetSystemLibrary.Delay` 1.0)
      (`GameplayStatics.PlaySoundAtLocation` "/Game/Audio/GruntsAndHits/SC_Death.SC_Death" (`self.K2_GetActorLocation`) (struct) 1.0 1.0 0.0 "/Game/Audio/SA_CharacterOverall.SA_CharacterOverall" null null null))))

(event `Play Sword Hits Sounds`
  ;[1 0.2874 0.9065] Play sword hit sounds
  (`GameplayStatics.PlaySoundAtLocation` "/Game/Audio/Sword_Hits/MS_SwordHit.MS_SwordHit" (`self.K2_GetActorLocation` (`self.GetOwner`)) (struct) 1.0 1.0 0.0 null null null null))

(event `self.ReceiveAnyDamage`
  (params (Damage :type "Float (single-precision)") (DamageType :type "DamageType Object Reference") (InstigatedBy :type "Controller Object Reference") (DamageCauser :type "Actor Object Reference"))
  ;[0.7299 0.4996 1] Making the character move after it has been hit
  (`self.Stop Combo`)
  (`self.PlayAnimMontage` (`|GetArrayItem` (`self.Hit Anims`) (`KismetMathLibrary.RandomIntegerInRange` 0 (- (`KismetArrayLibrary.Array_Length` (`self.Hit Anims`)) 1))))
  (bind _asbp_third_person_character (cast `/Game/ThirdPerson/Blueprints/BP_ThirdPersonCharacter` (`GameplayStatics.GetPlayerCharacter` 0)))
  (`self.LaunchCharacter` (* (`KismetMathLibrary.GetForwardVector` (`self.K2_GetActorRotation` _asbp_third_person_character)) 700.0))
  (`GameplayStatics.PlaySoundAtLocation` "/Game/Audio/GruntsAndHits/416839__tonsil5__grunt1-death-pain.416839__tonsil5__grunt1-death-pain" (`self.K2_GetActorLocation`) (struct) 1.0 (`KismetMathLibrary.RandomFloatInRange` -1.5 1.3) 0.0 "/Game/Audio/SA_CharacterOverall.SA_CharacterOverall" null null null)
  (bind _isplayerdead (`/Game/Blueprints/BPC_PlayerStats.Decrease Health` (`self.BPC_PlayerStats`) Damage))
  (if _isplayerdead
    (`PrimitiveComponent.SetCollisionObjectType` (`self.Mesh`) "ECC_PhysicsBody")
    (`PrimitiveComponent.SetSimulatePhysics` (`self.Mesh`) true)
    (`GameplayStatics.PlaySoundAtLocation` "/Game/Audio/GruntsAndHits/SC_Death.SC_Death" (`self.K2_GetActorLocation`) (struct) 1.0 1.0 0.0 "/Game/Audio/SA_CharacterOverall.SA_CharacterOverall" null null null)
    (`SceneComponent.SetVisibility` (`self.Health Bar Widget`) false false)
    (`KismetSystemLibrary.Delay` 2.5)
    (`CharacterMovementComponent.SetMovementMode` (`self.CharacterMovement`) "MOVE_None" 0)
    (bind _asbp_third_person_character_2 (cast `/Game/ThirdPerson/Blueprints/BP_ThirdPersonCharacter` (`GameplayStatics.GetPlayerCharacter` 0)))
    (`/Game/Blueprints/ABPC_Quest.Eliminate Enemy` (`/Game/ThirdPerson/Blueprints/BP_ThirdPersonCharacter.ABPC_Quest` _asbp_third_person_character_2) self)))

(event `Enable Investigation Icon`
  (bind _investigate_widget (`self.Investigate Widget`))
  ;[1 1 1] Investigate icon
  (`/Engine/EditorBlueprintResources/StandardMacros.FlipFlop`
    (:`A`
      (`SceneComponent.SetVisibility` _investigate_widget true false))
    (:`B`
      (`SceneComponent.SetVisibility` _investigate_widget false false))))

(event `Attack 1`
  ;[1 0.8317 0.8929] Combo system
  ;;[0.5345 0.6157 1] Attack 1
  (`/Engine/EditorBlueprintResources/StandardMacros.DoOnce` false :!label _label
    (:`Completed`
      (`KismetSystemLibrary.Delay` 0.1)
      (`|PlayMontage` (`self.Mesh`) "/Game/Characters/RPG_Character/Locomotion_animations/SwordAttacks/Attack1_Montage.Attack1_Montage" (`self.Attack Animation Speed`)
        (:`then`
          (set `self.attack index` 1)
          (goto _label :!via `Reset`))))))

(event `Sword Attack Combo From BT`
  ;[1 0.8317 0.8929] Combo system
  ;;[0.7711 0.642 1] Attack input
  (if (`self.Can Attack`)
    (`self.SwordAttack`)))

(event `SwordAttack`
  ;[1 0.8317 0.8929] Combo system
  ;;[1 0 0.8433] Sword attack
  (if (`self.isAttacking?`)
    (set `self.save attack` true)
    (else
      (set `self.isAttacking?` true)
      ;;[1 0.4745 0.9179] Switching between attacks
      (switch `int` (`self.attack index`) :!label _label_2
        (:`0`
          (`self.Attack 1`))
        (:`1`
          (`self.Attack 2`))
        (:`2`
          (`self.Attack4`))))))

(event `Attack 2`
  ;[1 0.8317 0.8929] Combo system
  ;;[0.5345 0.6157 1] Attack 2
  (`/Engine/EditorBlueprintResources/StandardMacros.DoOnce` false :!label _label_3
    (:`Completed`
      (`KismetSystemLibrary.Delay` 0.1)
      (`|PlayMontage` (`self.Mesh`) "/Game/Characters/RPG_Character/Locomotion_animations/SwordAttacks/Attack2_Montage.Attack2_Montage" (`self.Attack Animation Speed`)
        (:`then`
          (set `self.attack index` 2)
          (goto _label_3 :!via `Reset`))))))

(event `Sword Attack Combo`
  ;[1 0.8317 0.8929] Combo system
  ;;[1 0 0.4139] Combo
  (if (`self.save attack`)
    (set `self.save attack` false)
    (goto _label_2)
    (else
      (`self.Stop Combo`))))

(event `Attack4`
  ;[1 0.8317 0.8929] Combo system
  ;;[0.5345 0.6157 1] Attack 4
  (`/Engine/EditorBlueprintResources/StandardMacros.DoOnce` false :!label _label_4
    (:`Completed`
      (`KismetSystemLibrary.Delay` 0.1)
      (`|PlayMontage` (`self.Mesh`) "/Game/Characters/RPG_Character/Locomotion_animations/SwordAttacks/Attack3_Montage.Attack3_Montage" (`self.Attack Animation Speed`)
        (:`then`
          (set `self.attack index` 4)
          (goto _label_4 :!via `Reset`))))))

(event `Stop Combo`
  ;[1 0.8317 0.8929] Combo system
  ;;[1 0 0.6488] reset attack combo
  (set `self.isAttacking?` false)
  (set `self.attack index` 0))

(event `Start sword trace`
  ;[1 0.4253 0.8704] Sword Trace
  (bind _returnvalue (`KismetSystemLibrary.K2_SetTimerDelegate` (delegate `Sword trace loop`) 0.001 true))
  (set `self.SwordTraceLoop` _returnvalue))

(event `Sword trace loop`
  ;[1 0.4253 0.8704] Sword Trace
  (bind (_outhit _returnvalue) (`KismetSystemLibrary.SphereTraceSingle` :`Start` (`SceneComponent.K2_GetComponentLocation` (`self.SwordTipPoint`)) :`End` (`SceneComponent.K2_GetComponentLocation` (`self.SwordBottomPoint`)) :`Radius` 14.0 :`TraceChannel` "TraceTypeQuery1" :`DrawDebugType` "ForDuration" :`DrawTime` 0.2))
  (if _returnvalue
    (bind (_bblockinghit _binitialoverlap _time _distance _location _impactpoint _normal _impactnormal _physmat _hitactor) (`GameplayStatics.BreakHitResult` _outhit))
    (if (`self.ActorHasTag` _hitactor "Damagable")
      (`/Engine/EditorBlueprintResources/StandardMacros.DoOnce` false :!label _label_5
        (:`Completed`
          (`GameplayStatics.ApplyDamage` _hitactor 25.0)
          (`GameplayStatics.PlayWorldCameraShake` "/Game/Blueprints/BP_SortHit_CameraShake.BP_SortHit_CameraShake_C" _location 0.0 2000.0)
          (`self.Play Sword Hits Sounds`)
          (`GameplayStatics.SpawnEmitterAtLocation` "/Game/Effects/Blood/P_Blood_Splat_Cone.P_Blood_Splat_Cone" _location (`KismetMathLibrary.MakeRotFromXY` _normal _normal) (0.4 0.4 0.4) true "AutoRelease")
          (`KismetSystemLibrary.Delay` 0.1)
          (goto _label_5 :!via `Reset`))))))

(event `Stop Sword Trace`
  ;[1 0.4253 0.8704] Sword Trace
  (`KismetSystemLibrary.K2_ClearAndInvalidateTimerHandle` (`self.SwordTraceLoop`)))

(event `Sphere Trace`
  (bind _returnvalue (`SceneComponent.K2_GetComponentLocation` (`self.SphereTrace`)))
  ;[0.9378 0.6936 1] Sphere Traced
  (bind (_outhit _returnvalue_2) (`KismetSystemLibrary.SphereTraceSingle` :`Start` _returnvalue :`End` _returnvalue :`Radius` 25.0 :`TraceChannel` "TraceTypeQuery1" :`DrawDebugType` "ForDuration"))
  (if _returnvalue_2
    (bind (_bblockinghit _binitialoverlap _time _distance _location _impactpoint _normal _impactnormal _physmat _hitactor) (`GameplayStatics.BreakHitResult` _outhit))
    (if (`self.ActorHasTag` _hitactor "Damagable")
      (`GameplayStatics.ApplyDamage` _hitactor 10.0)
      (`GameplayStatics.PlayWorldCameraShake` "/Game/Blueprints/BP_SortHit_CameraShake.BP_SortHit_CameraShake_C" _location 0.0 2000.0)
      (`self.Play Sword Hits Sounds`)
      ;;[1 1 1] Lost Blood texture
      (`GameplayStatics.SpawnEmitterAtLocation` "/Game/Effects/Blood/P_Blood_Splat_Cone.P_Blood_Splat_Cone" _location (`KismetMathLibrary.MakeRotFromXY` _normal _normal) (0.4 0.4 0.4) true "AutoRelease"))))

(fn `Attack`
  (returns (AnimationDuration :type "Float (double-precision)"))
  (`self.Sword Attack Combo From BT`)
  (return 0.4))

(fn `StealthBackKill`
  (returns (`Ref Location` :type "Vector Structure") (`Assassin Rotation` :type "Rotator Structure"))
  (`self.PlayAnimMontage` "/Game/Characters/RPG_Character/Locomotion_animations/Stealth/Paired_Knife_Stealth_KidneyAndNeck_Vic_Montage.Paired_Knife_Stealth_KidneyAndNeck_Vic_Montage")
  (`self.RagDoll`)
  (`SceneComponent.SetVisibility` (`self.Kill Widget`) false false)
  (`SceneComponent.SetVisibility` (`self.Health Bar Widget`) false false)
  (`CharacterMovementComponent.SetMovementMode` (`self.CharacterMovement`) "MOVE_None" 0)
  (return (`SceneComponent.K2_GetComponentLocation` (`self.As_ Reference`)) (`self.K2_GetActorRotation`)))

(fn `UserConstructionScript`)