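; BP_AIController_Boss is the AI controller for a boss enemy, driving its behavior and managing the on-screen boss health bar.
; On BeginPlay it runs the BT_AI_Boss behavior tree.
; ActivateBossCombat creates a WB_BossHealthBar widget, stores it and adds it to the viewport.
; DeactivateBossCombat removes that widget if it is valid and clears the reference.
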(event `self.ReceiveBeginPlay`
  (`self.RunBehaviorTree` "/Game/AI/Boss/BT_AI_Boss.BT_AI_Boss"))

(event `Activate Boss Combat`
  (bind _returnvalue (`|CreateWidget` "/Game/UI/WB_BossHealthBar.WB_BossHealthBar_C"))
  (bind _output_get (set `self.Boss Health Bar Widget` _returnvalue))
  (`UserWidget.AddToViewport` _output_get 0))

(event `Deactivate Boss Combat`
  (bind _boss_health_bar_widget (`self.Boss Health Bar Widget`)
    (:`then`
      (`Widget.RemoveFromParent` _boss_health_bar_widget)
      (set `self.Boss Health Bar Widget` null))
    (:`else`)))

(fn `UserConstructionScript`
  (`parent.UserConstructionScript`))