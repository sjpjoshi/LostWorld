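; Actor component that drives the on-screen quest HUD for the active quest.
; On BeginPlay it creates a WB_EmitQuestHud widget, stores it and adds it to the viewport.
; Separate events push the ActiveQuest's name into the widget's CurrentQuest text and pass its objectives to the widget's FillObjectives.
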(event `self.ReceiveBeginPlay`
  ;[1 0.4844 0.8711] Adds active quest to the screen
  (bind _returnvalue (`|CreateWidget` "/Game/UI/WB_EmitQuestHud.WB_EmitQuestHud_C"))
  (bind _output_get (set `self.Quest HUD Widget` _returnvalue))
  (`UserWidget.AddToViewport` _output_get 0))

(event `Set Active Quest Text`
  ;[1 0.4947 0.5646] Sets the active quest
  (`TextBlock.SetText` (`/Game/UI/WB_EmitQuestHud.CurrentQuest` (`self.Quest HUD Widget`)) (`KismetTextLibrary.Conv_StringToText` (`.QuestName_2_DA12041E4E114A56EF5919B95D8D57B4` (break `/Game/quest_system/S_Quest` (`self.active quest`))))))

(event `Set Objectives`
  (bind (_active_quest_questname _active_quest_questdescription _active_quest_secondary _active_quest_completed _active_quest_objectives) (break `/Game/quest_system/S_Quest` (`self.active quest`)))
  ;[0.4003 0.8283 1] Setting the objectives
  (`/Game/UI/WB_EmitQuestHud.Fill Objectives` (`self.Quest HUD Widget`) _active_quest_objectives))