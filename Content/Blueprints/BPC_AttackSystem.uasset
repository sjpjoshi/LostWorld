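; Melee attack component for the third-person character, running a four-step combo of sword montages with a kick as the third step.
; Attack input starts the chain or buffers a press, which SwordAttackCombo uses to play the next montage by AttackIndex or reset.
; A looping timer sphere-traces along the blade, with a separate single-point SphereTrace event.
; Both damage "Damagable" actors with camera shake and sound, and blade hits have a cooldown.
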(event `self.ReceiveBeginPlay`
  ;[0 0.7618 1] getting the character mesh
  (bind _asbp_third_person_character (cast `/Game/ThirdPerson/Blueprints/BP_ThirdPersonCharacter` (`self.GetOwner`)))
  (set `self.Character BP` _asbp_third_person_character)
  (set `self.Character Mesh` (`Character.Mesh` _asbp_third_person_character)))

(event `Start sword trace`
  ;[1 0.4253 0.8704] Sword Trace
  (bind _returnvalue (`KismetSystemLibrary.K2_SetTimerDelegate` (delegate `Sword trace loop`) 0.001 true))
  (set `self.SwordTraceLoop` _returnvalue))

(event `Attack 1`
  ;[1 0.8317 0.8929] Combo system
  ;;[0.5345 0.6157 1] Attack 1
  (`/Engine/EditorBlueprintResources/StandardMacros.DoOnce` false :!label _label
    (:`Completed`
      (`KismetSystemLibrary.Delay` 0.1)
      (`|PlayMontage` (`self.Character Mesh`) "/Game/Characters/RPG_Character/Locomotion_animations/SwordAttacks/Attack1_Montage.Attack1_Montage"
        (:`then`
          (set `self.attack index` 1)
          (goto _label :!via `Reset`))))))

(event `InputAction|Attack`
  (params (Key :type "Key Structure"))
  ;[1 0.8317 0.8929] Combo system
  ;;[0.7711 0.642 1] Attack input
  (:`Pressed`
    (if (`self.canAttack`)
      (`self.SwordAttack`))))

(event `Sword trace loop`
  ;[1 0.4253 0.8704] Sword Trace
  (bind (_outhit _returnvalue) (`KismetSystemLibrary.SphereTraceSingle` :`Start` (`SceneComponent.K2_GetComponentLocation` (`/Game/ThirdPerson/Blueprints/BP_ThirdPersonCharacter.SwordTipPoint` (`self.Character BP`))) :`End` (`SceneComponent.K2_GetComponentLocation` (`/Game/ThirdPerson/Blueprints/BP_ThirdPersonCharacter.SwordBottomPoint` (`self.Character BP`))) :`Radius` 12.0 :`TraceChannel` "TraceTypeQuery1" :`DrawDebugType` "ForDuration" :`DrawTime` 0.2))
  (if _returnvalue
    (bind (_bblockinghit _binitialoverlap _time _distance _location _impactpoint _normal _impactnormal _physmat _hitactor) (`GameplayStatics.BreakHitResult` _outhit))
    (if (`Actor.ActorHasTag` _hitactor "Damagable")
      (`/Engine/EditorBlueprintResources/StandardMacros.DoOnce` false :!label _label_2
        (:`Completed`
          (`GameplayStatics.ApplyDamage` _hitactor 10.0)
          (`GameplayStatics.PlayWorldCameraShake` "/Game/Blueprints/BP_SortHit_CameraShake.BP_SortHit_CameraShake_C" _location 0.0 2000.0)
          (`self.Play Sword Hits Sounds`)
          (`KismetSystemLibrary.Delay` 0.5)
          (goto _label_2 :!via `Reset`))))))

(event `Attack 2`
  ;[1 0.8317 0.8929] Combo system
  ;;[0.5345 0.6157 1] Attack 2
  (`/Engine/EditorBlueprintResources/StandardMacros.DoOnce` false :!label _label_3
    (:`Completed`
      (`KismetSystemLibrary.Delay` 0.1)
      (`|PlayMontage` (`self.Character Mesh`) "/Game/Characters/RPG_Character/Locomotion_animations/SwordAttacks/Attack2_Montage.Attack2_Montage"
        (:`then`
          (set `self.attack index` 2)
          (goto _label_3 :!via `Reset`))))))

(event `SwordAttack`
  ;[1 0.8317 0.8929] Combo system
  ;;[1 0 0.8433] Sword attack
  (if (`self.isAttacking?`)
    (set `self.save attack` true)
    (else
      (set `self.isAttacking?` true)
      ;;[1 0.4745 0.9179] Switching between attacks
      (switch `int` (`self.attack index`) :!label _label_4
        (:`0`
          (`self.Attack 1`))
        (:`1`
          (`self.Attack 2`))
        (:`2`
          (`self.Attack 3`))
        (:`3`
          (`self.Attack4`))))))

(event `Stop Sword Trace`
  ;[1 0.4253 0.8704] Sword Trace
  (`KismetSystemLibrary.K2_ClearAndInvalidateTimerHandle` (`self.SwordTraceLoop`)))

(event `Sword Attack Combo`
  ;[1 0.8317 0.8929] Combo system
  ;;[1 0 0.4139] Combo
  (if (`self.save attack`)
    (set `self.save attack` false)
    (goto _label_4)
    (else
      (`self.Stop Combo`))))

(event `Attack 3`
  ;[1 0.8317 0.8929] Combo system
  ;;[0.5345 0.6157 1] Attack 3
  (`/Engine/EditorBlueprintResources/StandardMacros.DoOnce` false :!label _label_5
    (:`Completed`
      (`KismetSystemLibrary.Delay` 0.1)
      (`|PlayMontage` (`self.Character Mesh`) "/Game/Characters/RPG_Character/Locomotion_animations/SwordAttacks/Kick_Montage.Kick_Montage"
        (:`then`
          (set `self.attack index` 3)
          (goto _label_5 :!via `Reset`))))))

(event `Sphere Trace`
  (bind _returnvalue (`SceneComponent.K2_GetComponentLocation` (`/Game/ThirdPerson/Blueprints/BP_ThirdPersonCharacter.SphereTrace` (`self.Character BP`))))
  (bind (_outhit _returnvalue_2) (`KismetSystemLibrary.SphereTraceSingle` :`Start` _returnvalue :`End` _returnvalue :`Radius` 25.0 :`TraceChannel` "TraceTypeQuery1" :`DrawDebugType` "ForDuration"))
  (if _returnvalue_2
    (bind (_bblockinghit _binitialoverlap _time _distance _location _impactpoint _normal _impactnormal _physmat _hitactor) (`GameplayStatics.BreakHitResult` _outhit))
    (if (`Actor.ActorHasTag` _hitactor "Damagable")
      (`GameplayStatics.ApplyDamage` _hitactor 10.0)
      (`GameplayStatics.PlayWorldCameraShake` "/Game/Blueprints/BP_SortHit_CameraShake.BP_SortHit_CameraShake_C" _location 0.0 2000.0)
      (`self.Play Sword Hits Sounds`))))

(event `Stop Combo`
  ;[1 0.8317 0.8929] Combo system
  ;;[1 0 0.6488] reset attack combo
  (set `self.isAttacking?` false)
  (set `self.attack index` 0))

(event `Attack4`
  ;[1 0.8317 0.8929] Combo system
  ;;[0.5345 0.6157 1] Attack 4
  (`/Engine/EditorBlueprintResources/StandardMacros.DoOnce` false :!label _label_6
    (:`Completed`
      (`KismetSystemLibrary.Delay` 0.1)
      (`|PlayMontage` (`self.Character Mesh`) "/Game/Characters/RPG_Character/Locomotion_animations/SwordAttacks/Attack3_Montage.Attack3_Montage"
        (:`then`
          (set `self.attack index` 4)
          (goto _label_6 :!via `Reset`))))))

(event `Play Sword Hits Sounds`
  ;[1 0.2874 0.9065] Play sword hit sounds
  (`GameplayStatics.PlaySoundAtLocation` "/Game/Audio/Sword_Hits/MS_SwordHit.MS_SwordHit" (`Actor.K2_GetActorLocation` (`self.GetOwner`)) (struct) 1.0 1.0 0.0 null null null null))