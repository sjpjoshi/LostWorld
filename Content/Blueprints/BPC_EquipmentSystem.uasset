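; Equipment component for BP_ThirdPersonCharacter that collects weapons and toggles an equipment menu.
; Interact sphere-traces forward from the follow camera, appends a hit BP_Weapon's item data to WeaponSlots and destroys the actor.
; The menu input lazily creates then shows or hides WB_Equipment, switching cursor, input mode, movement and the attack system's CanAttack.
; The H key prints stored weapon row names for debugging.
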(event `self.ReceiveBeginPlay`
  (bind _asbp_third_person_character (cast `/Game/ThirdPerson/Blueprints/BP_ThirdPersonCharacter` (`self.GetOwner`)))
  (set `self.Follow Camera` (`/Game/ThirdPerson/Blueprints/BP_ThirdPersonCharacter.FollowCamera` _asbp_third_person_character))
  (set `self.BPC Attack System` (`/Game/ThirdPerson/Blueprints/BP_ThirdPersonCharacter.BPC_AttackSystem` _asbp_third_person_character)))

(event `InputAction|Interact`
  (params (Key :type "Key Structure"))
  (bind _follow_camera (`self.Follow Camera`))
  (bind _returnvalue (`SceneComponent.K2_GetComponentLocation` _follow_camera))
  ;[1 1 1] Pick Up trace
  (:`Pressed`
    (bind (_outhit _returnvalue_2) (`KismetSystemLibrary.SphereTraceSingleForObjects` :`Start` _returnvalue :`End` (+ _returnvalue (* (`KismetMathLibrary.GetForwardVector` (`SceneComponent.K2_GetComponentRotation` _follow_camera)) 1000.0)) :`Radius` 10.0 :`ObjectTypes` (`|MakeArray` "ObjectTypeQuery2" :!type "EObjectTypeQuery Enum") :`DrawDebugType` "ForDuration"))
    (if _returnvalue_2
      (bind _asbp_weapon (cast `/Game/Blueprints/BP_Weapon` (`.HitActor` (`GameplayStatics.BreakHitResult` _outhit)))
        (:`then`
          (`self.Add Weapon` (`/Game/Blueprints/BP_Weapon.item data` _asbp_weapon)))
        (:`CastFailed`
          _))
      (`Actor.K2_DestroyActor` _asbp_weapon)
      (`KismetSystemLibrary.PrintText` "collected"))))

(event `Key|H`
  (params (Key :type "Key Structure"))
  ;[1 1 1] Pick Up trace
  (:`Pressed`
    (for _array_element (`self.Weapon Slots`)
      (`KismetSystemLibrary.PrintText` (`KismetTextLibrary.Conv_NameToText` (`.RowName` (break `DataTableRowHandle` (break `/Game/Equipment_System/S_Slots` _array_element))))))))

(event `InputAction|EquipmentMenu`
  (params (Key :type "Key Structure"))
  (bind _returnvalue (`GameplayStatics.GetPlayerController` 0))
  (bind _bpc_attack_system (`self.BPC Attack System`))
  ;[1 1 1] Equipment Menu Panel
  (:`Pressed`
    (if (not (`self.isPanelOpen`))
      (set `/Game/Blueprints/BPC_AttackSystem.canAttack` false _bpc_attack_system)
      (set `self.isPanelOpen` true)
      (bind _equipment_widget (`self.Equipment Widget`)
        (:`then`
          (`Widget.SetVisibility` _equipment_widget "Visible"))
        (:`else`
          (bind _returnvalue_2 (`|CreateWidget` "/Game/Blueprints/UI/WB_Equipment.WB_Equipment_C"))
          (bind _output_get (set `self.Equipment Widget` _returnvalue_2))
          (`UserWidget.AddToViewport` _output_get 0)))
      (set `PlayerController.bShowMouseCursor` true _returnvalue)
      (`WidgetBlueprintLibrary.SetInputMode_GameAndUIEx` _returnvalue (`self.Equipment Widget`))
      (bind _asbp_third_person_character (cast `/Game/ThirdPerson/Blueprints/BP_ThirdPersonCharacter` (`self.GetOwner`)))
      (`CharacterMovementComponent.SetMovementMode` (`Character.CharacterMovement` _asbp_third_person_character) "MOVE_None" 0)
      (else
        (set `/Game/Blueprints/BPC_AttackSystem.canAttack` true _bpc_attack_system)
        (set `self.isPanelOpen` false)
        (bind _equipment_widget_2 (`self.Equipment Widget`)
          (:`then`
            (`Widget.SetVisibility` _equipment_widget_2 "Hidden")
            (set `PlayerController.bShowMouseCursor` false _returnvalue)
            (`WidgetBlueprintLibrary.SetInputMode_GameOnly` _returnvalue)
            (bind _asbp_third_person_character_2 (cast `/Game/ThirdPerson/Blueprints/BP_ThirdPersonCharacter` (`self.GetOwner`)))
            (`CharacterMovementComponent.SetMovementMode` (`Character.CharacterMovement` _asbp_third_person_character_2) "MOVE_Walking" 0))
          (:`else`))))))

(fn `Add Weapon`
  (params (NewItem :type "/Game/Equipment_System/S_Slots Structure (by ref)"))
  (`KismetArrayLibrary.Array_Add` (`self.Weapon Slots`) NewItem))