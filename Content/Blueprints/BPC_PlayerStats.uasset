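; Stats component that tracks health, stamina, XP and level for the player character, and health for BP_Dummy.
; One tick after BeginPlay it identifies its owner and fills the matching HUD or health bar.
; Stat functions push changes straight to widgets, with only setup and DecreaseHealth supporting the dummy.
; Reaching max XP triggers IncreaseLevel, which raises the threshold, resets XP and plays sounds above level zero.
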(event `self.ReceiveBeginPlay`
  (bind _hud_widget (`/Game/ThirdPerson/Blueprints/BP_ThirdPersonCharacter.HUD Widget` (`self.Player Character BP`)))
  (`KismetSystemLibrary.DelayUntilNextTick`)
  (bind _asbp_third_person_character (cast `/Game/ThirdPerson/Blueprints/BP_ThirdPersonCharacter` (`self.GetOwner`))
    (:`then`
      (set `self.Player Character BP` _asbp_third_person_character)
      (set `self.isPlayer?` true)
      (`ProgressBar.SetPercent` (`/Game/UI/WB_HUD.StaminaBar` _hud_widget) (/ (`self.currentStamina`) (`self.maxStamina`)))
      (`TextBlock.SetText` (`/Game/UI/WB_HUD.StaminaText` _hud_widget) (`KismetTextLibrary.Conv_DoubleToText` (`self.currentStamina`) "HalfToEven"))
      (`self.IncreaseLevel` 0)
      (`ProgressBar.SetPercent` (`/Game/UI/WB_HUD.XPBar` (`/Game/ThirdPerson/Blueprints/BP_ThirdPersonCharacter.HUD Widget` (`self.Player Character BP`))) (/ (`self.XP`) (`self.maxXP`)))
      (`TextBlock.SetText` (`/Game/UI/WB_HUD.XPText` (`/Game/ThirdPerson/Blueprints/BP_ThirdPersonCharacter.HUD Widget` (`self.Player Character BP`))) (`|FormatText` "{CurrentXP} / {Max XP}" (`self.XP`) (`self.maxXP`)))
      (`TextBlock.SetText` (`/Game/UI/WB_HUD.LevelText` (`/Game/ThirdPerson/Blueprints/BP_ThirdPersonCharacter.HUD Widget` (`self.Player Character BP`))) (`KismetTextLibrary.Conv_IntToText` (`self.Level`))))
    (:`CastFailed`
      (bind _asbp_dummy (cast `/Game/Blueprints/BP_Dummy` (`self.GetOwner`)))
      (set `self.BP Dummy` _asbp_dummy)
      (set `self.isPlayer?` false)))
  (`ProgressBar.SetPercent` (select `bool` (`self.isPlayer?`) :`false` (`/Game/UI/WB_DummyHealthBar.HealthBar` (`/Game/Blueprints/BP_Dummy.Health Bar UI` (`self.BP Dummy`))) :`true` (`/Game/UI/WB_HUD.Healthbar` (`/Game/ThirdPerson/Blueprints/BP_ThirdPersonCharacter.HUD Widget` (`self.Player Character BP`)))) (/ (`self.currentHealth`) (`self.maxHealth`)))
  (`TextBlock.SetText` (select `bool` (`self.isPlayer?`) :`false` (`/Game/UI/WB_DummyHealthBar.HealthText` (`/Game/Blueprints/BP_Dummy.Health Bar UI` (`self.BP Dummy`))) :`true` (`/Game/UI/WB_HUD.HealthText` (`/Game/ThirdPerson/Blueprints/BP_ThirdPersonCharacter.HUD Widget` (`self.Player Character BP`)))) (`KismetTextLibrary.Conv_DoubleToText` (`self.currentHealth`) "HalfToEven")))

(fn `Decrease Health`
  (params (Damage :type "Float (double-precision)"))
  (returns (IsPlayerDead :type Boolean))
  ;[1 0.03805 0.321] Health Decrease
  (if (not (<= (`self.currentHealth`) 0.0))
    (bind _output_get (set `self.currentHealth` (- (`self.currentHealth`) Damage)))
    (`ProgressBar.SetPercent` (select `bool` (`self.isPlayer?`) :`false` (`/Game/UI/WB_DummyHealthBar.HealthBar` (`/Game/Blueprints/BP_Dummy.Health Bar UI` (`self.BP Dummy`))) :`true` (`/Game/UI/WB_HUD.Healthbar` (`/Game/ThirdPerson/Blueprints/BP_ThirdPersonCharacter.HUD Widget` (`self.Player Character BP`)))) (/ _output_get (`self.maxHealth`)))
    (`TextBlock.SetText` (select `bool` (`self.isPlayer?`) :`false` (`/Game/UI/WB_DummyHealthBar.HealthText` (`/Game/Blueprints/BP_Dummy.Health Bar UI` (`self.BP Dummy`))) :`true` (`/Game/UI/WB_HUD.HealthText` (`/Game/ThirdPerson/Blueprints/BP_ThirdPersonCharacter.HUD Widget` (`self.Player Character BP`)))) (`KismetTextLibrary.Conv_DoubleToText` (`self.currentHealth`) "HalfToEven"))
    (if (<= (`self.currentHealth`) 0.0)
      _
      (else
        (return false))))
  (return true))

(fn `Decrease Stamina`
  (params (`Stamina Depleted` :type "Float (double-precision)"))
  (returns (StaminaLeft :type Boolean))
  (bind _hud_widget (`/Game/ThirdPerson/Blueprints/BP_ThirdPersonCharacter.HUD Widget` (`self.Player Character BP`)))
  ;[1 0.211 0.8379] Stamina Decrease
  (if (not (<= (`self.currentStamina`) 0.0))
    (bind _output_get (set `self.currentStamina` (- (`self.currentStamina`) `Stamina Depleted`)))
    (`ProgressBar.SetPercent` (`/Game/UI/WB_HUD.StaminaBar` _hud_widget) (/ _output_get (`self.maxStamina`)))
    (`TextBlock.SetText` (`/Game/UI/WB_HUD.StaminaText` _hud_widget) (`KismetTextLibrary.Conv_DoubleToText` (`self.currentStamina`) "HalfToEven"))
    (if (<= 0.0 (`self.currentStamina`))
      _
      (else
        (return true))))
  (return false))

(fn `Increase Health`
  (params (AddedHealth :type "Float (double-precision)"))
  (bind _hud_widget (`/Game/ThirdPerson/Blueprints/BP_ThirdPersonCharacter.HUD Widget` (`self.Player Character BP`)))
  (set `self.currentHealth` (+ (`self.currentHealth`) AddedHealth))
  (if (> (`self.currentHealth`) (`self.maxHealth`))
    (bind _output_get (set `self.currentHealth` (`self.maxHealth`))))
  (`ProgressBar.SetPercent` (`/Game/UI/WB_HUD.Healthbar` _hud_widget) (/ _output_get (`self.maxHealth`)))
  (`TextBlock.SetText` (`/Game/UI/WB_HUD.HealthText` _hud_widget) (`KismetTextLibrary.Conv_DoubleToText` (`self.currentHealth`) "HalfToEven")))

(fn `Increase Max Health`
  (params (`Health Incremention ` :type "Float (double-precision)"))
  (bind _hud_widget (`/Game/ThirdPerson/Blueprints/BP_ThirdPersonCharacter.HUD Widget` (`self.Player Character BP`)))
  (set `self.maxHealth` (+ `Health Incremention ` (`self.maxHealth`)))
  (`ProgressBar.SetPercent` (`/Game/UI/WB_HUD.Healthbar` _hud_widget) (/ (`self.currentHealth`) (`self.maxHealth`)))
  (`TextBlock.SetText` (`/Game/UI/WB_HUD.HealthText` _hud_widget) (`KismetTextLibrary.Conv_DoubleToText` (`self.currentHealth`) "HalfToEven")))

(fn `Increase Max Stamina`
  (params (AddStamina :type "Float (double-precision)"))
  (bind _hud_widget (`/Game/ThirdPerson/Blueprints/BP_ThirdPersonCharacter.HUD Widget` (`self.Player Character BP`)))
  (set `self.maxStamina` (+ AddStamina (`self.currentStamina`)))
  (`ProgressBar.SetPercent` (`/Game/UI/WB_HUD.StaminaBar` _hud_widget) (/ (`self.currentStamina`) (`self.maxStamina`)))
  (`TextBlock.SetText` (`/Game/UI/WB_HUD.StaminaText` _hud_widget) (`KismetTextLibrary.Conv_DoubleToText` (`self.currentStamina`) "HalfToEven")))

(fn `Increase Stamina`
  (params (AddedStamina :type "Float (double-precision)"))
  (bind _hud_widget (`/Game/ThirdPerson/Blueprints/BP_ThirdPersonCharacter.HUD Widget` (`self.Player Character BP`)))
  (set `self.currentStamina` (+ AddedStamina (`self.currentStamina`)))
  (if (> (`self.currentStamina`) (`self.maxStamina`))
    (set `self.currentStamina` (`self.maxStamina`)))
  (`ProgressBar.SetPercent` (`/Game/UI/WB_HUD.StaminaBar` _hud_widget) (/ (`self.currentStamina`) (`self.maxStamina`)))
  (`TextBlock.SetText` (`/Game/UI/WB_HUD.StaminaText` _hud_widget) (`KismetTextLibrary.Conv_DoubleToText` (`self.currentStamina`) "HalfToEven")))

(fn `IncreaseLevel`
  (params (AddedLevel :type Integer))
  (set `self.Level` (+ (`self.Level`) AddedLevel))
  (set `self.maxXP` (+ (`self.maxXP`) 150.0))
  (set `self.XP` 0.0)
  (`TextBlock.SetText` (`/Game/UI/WB_HUD.LevelText` (`/Game/ThirdPerson/Blueprints/BP_ThirdPersonCharacter.HUD Widget` (`self.Player Character BP`))) (`KismetTextLibrary.Conv_IntToText` (`self.Level`)))
  (if (> (`self.Level`) 0)
    (`GameplayStatics.PlaySound2D` "/Game/Audio/UI/475889__epicsoundeffects__ese-whoosh-epic-level-up.475889__epicsoundeffects__ese-whoosh-epic-level-up" 1.0 1.0 0.0 null null)
    (`GameplayStatics.PlaySound2D` "/Game/Audio/UI/542825__kostas17__magic-spell.542825__kostas17__magic-spell" 1.0 1.0 0.0 null null)))

(fn `IncreaseXP`
  (params (AddedXP :type "Float (double-precision)"))
  (set `self.XP` (+ (`self.XP`) AddedXP))
  (if (>= (`self.XP`) (`self.maxXP`))
    (`self.IncreaseLevel` 1))
  (`ProgressBar.SetPercent` (`/Game/UI/WB_HUD.XPBar` (`/Game/ThirdPerson/Blueprints/BP_ThirdPersonCharacter.HUD Widget` (`self.Player Character BP`))) (/ (`self.XP`) (`self.maxXP`)))
  (`TextBlock.SetText` (`/Game/UI/WB_HUD.XPText` (`/Game/ThirdPerson/Blueprints/BP_ThirdPersonCharacter.HUD Widget` (`self.Player Character BP`))) (`|FormatText` "{CurrentXP} / {Max XP}" (`self.XP`) (`self.maxXP`))))