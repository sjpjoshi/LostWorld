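; BP_Quest_Giver is an interactable quest giver that plays dialogue and then presents its list of quests.
; A trigger radius toggles an interact widget for the player character, and Tick turns that widget toward the camera.
; Each Interact advances the Dialogue array, then opens a quest widget filled from Quests with a back-reference to the giver.
; Interacting again or CloseWidget removes it and restores game-only input.
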(event `self.ReceiveTick`
  (params (DeltaSeconds :type "Float (single-precision)"))
  ;[0 0.2755 1] Setting rotation
  (`SceneComponent.K2_SetWorldRotation` (`self.Interact Widget`) (`KismetMathLibrary.FindLookAtRotation` (`SceneComponent.K2_GetComponentLocation` (`self.Interact Widget`)) (`SceneComponent.K2_GetComponentLocation` (`PlayerCameraManager.TransformComponent` (`GameplayStatics.GetPlayerCameraManager` 0)))) false false))

(event `self.TriggerRadius.OnComponentBeginOverlap`
  (params (OverlappedComponent :type "PrimitiveComponent Object Reference") (OtherActor :type "Actor Object Reference") (OtherComp :type "PrimitiveComponent Object Reference") (OtherBodyIndex :type Integer) (bFromSweep :type Boolean) (SweepResult :type "HitResult Structure (by ref)"))
  ;[0.2601 0.5652 1] Setting visibility when dead
  (cast `/Game/ThirdPerson/Blueprints/BP_ThirdPersonCharacter` OtherActor)
  (`SceneComponent.SetVisibility` (`self.Interact Widget`) true false))

(event `self.TriggerRadius.OnComponentEndOverlap`
  (params (OverlappedComponent :type "PrimitiveComponent Object Reference") (OtherActor :type "Actor Object Reference") (OtherComp :type "PrimitiveComponent Object Reference") (OtherBodyIndex :type Integer))
  ;[0.2601 0.5652 1] Setting visibility when dead
  (cast `/Game/ThirdPerson/Blueprints/BP_ThirdPersonCharacter` OtherActor)
  (`SceneComponent.SetVisibility` (`self.Interact Widget`) false false))

(event `/Game/quest_system/BPI_QuestGiver.Interact`
  (bind _returnvalue (`GameplayStatics.GetPlayerController` 0))
  (bind _returnvalue_2 (`GameplayStatics.GetPlayerController` 0))
  (bind _dialogueindex (`self.dialogueIndex`))
  ;[0.3953 0.5746 1] Quest
  (if (not (`self.Widget Active`))
    (if (not (`self.dialogueOpened`))
      (bind _returnvalue_3 (`|CreateWidget` "/Game/quest_system/WB_QuestGiverDialogue.WB_QuestGiverDialogue_C"))
      (bind _output_get (set `self.dialogueWidget` _returnvalue_3))
      (`UserWidget.AddToViewport` _output_get 0)
      (set `self.dialogueOpened` true)
      (`TextBlock.SetText` (`/Game/quest_system/WB_QuestGiverDialogue.DialogueText` (`self.dialogueWidget`)) (`KismetTextLibrary.Conv_StringToText` (`|GetArrayItem` (`self.Dialogue`) (`self.dialogueIndex`))))
      (`/Engine/EditorBlueprintResources/StandardMacros.IncrementInt` (`self.dialogueIndex`)
        (:`  `
          (set `PlayerController.bShowMouseCursor` true _returnvalue_2)
          (`WidgetBlueprintLibrary.SetInputMode_GameAndUIEx` _returnvalue_2 (`self.Quest Widget`))))
      (else
        (`TextBlock.SetText` (`/Game/quest_system/WB_QuestGiverDialogue.DialogueText` (`self.dialogueWidget`)) (`KismetTextLibrary.Conv_StringToText` (`|GetArrayItem` (`self.Dialogue`) (`self.dialogueIndex`))))
        (`/Engine/EditorBlueprintResources/StandardMacros.IncrementInt` _dialogueindex
          (:`  `
            (if (> _dialogueindex (`KismetArrayLibrary.Array_Length` (`self.Dialogue`)))
              (`Widget.RemoveFromParent` (`self.dialogueWidget`))
              (set `self.dialogueOpened` false)
              (set `self.dialogueIndex` 0)
              (set `self.dialogueWidget` null)
              (`self.Open Quest Widget`))))))
    (else
      (`Widget.RemoveFromParent` (`self.Quest Widget`) :!label _label)
      (set `self.Quest Widget` null)
      (set `PlayerController.bShowMouseCursor` false _returnvalue)
      (`WidgetBlueprintLibrary.SetInputMode_GameOnly` _returnvalue)
      (set `self.Widget Active` false))))

(event `Open Quest Widget`
  ;[0.3953 0.5746 1] Quest
  (bind _returnvalue (`|CreateWidget` "/Game/quest_system/WB_QuestGiver.WB_QuestGiver_C"))
  (bind _output_get (set `self.Quest Widget` _returnvalue))
  (`UserWidget.AddToViewport` _output_get 0)
  (set `self.Widget Active` true)
  (set `/Game/quest_system/WB_QuestGiver.Quest Giver BluePrint` self (`self.Quest Widget`))
  (for _array_element (`self.Quests`)
    (`/Game/quest_system/WB_QuestGiver.Add Quest` (`self.Quest Widget`) _array_element)))

(event `Close Widget`
  ;[0.3953 0.5746 1] Quest
  (goto _label))

(fn `UserConstructionScript`)